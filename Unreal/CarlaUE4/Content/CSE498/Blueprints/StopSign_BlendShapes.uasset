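; StopSign_BlendShapes is a stop sign Blueprint that randomly appears bent, using a morph target on its skeletal mesh.
; On BeginPlay, a random roll against BentChance decides whether MorphTargetValue gets a random amount between the minimum and maximum bend settings.
; Tick reapplies that value to the "Bent" morph target every frame, although it is only randomized at BeginPlay.
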(event `self.ReceiveBeginPlay`
  (`/Engine/EditorBlueprintResources/StandardMacros.CompareFloat` (`KismetMathLibrary.RandomFloat`) (`self.BentChance`)
    (:`<`
      (set `self.MorphTargetValue` (`KismetMathLibrary.RandomFloatInRange` (`self.MinBentAmount`) (`self.MaxBentAmount`))))))

(event `self.ReceiveTick`
  (params (DeltaSeconds :type "Float (single-precision)"))
  (`SkeletalMeshComponent.SetMorphTarget` (`self.SkeletalMesh`) "Bent" (`self.MorphTargetValue`) true))

(fn `UserConstructionScript`)
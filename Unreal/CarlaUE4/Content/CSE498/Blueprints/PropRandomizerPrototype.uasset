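; Prototype prop randomizer Blueprint that jitters the transforms of every BP_StreetLight_simple_LB actor in the level.
; RandomizePropTransforms sets each light's mesh to Movable, then applies random offsets to location, rotation and scale, interpolated between min/max variables.
; Changes build on current transforms, so repeated runs accumulate; rotation deltas come from MakeRotationFromAxes rather than Euler angles.
; The event graph and construction script are empty, so nothing here calls the function.
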(fn `RandomizePropTransforms`
  (bind (_x _y _z) (`KismetMathLibrary.BreakRotIntoAxes` (`self.RotationRandomizationMin`)))
  (bind (_x_2 _y_2 _z_2) (`KismetMathLibrary.BreakRotIntoAxes` (`self.RotationRandomizationMax`)))
  (bind _outactors (`GameplayStatics.GetAllActorsOfClass` "/Game/Carla/Static/StreetLight/BP_StreetLight_simple_LB.BP_StreetLight_simple_LB_C"))
  (for _array_element _outactors
    (`SceneComponent.SetMobility` (`/Game/Carla/Static/StreetLight/BP_StreetLight_simple_LB.StreetLight_Mesh` _array_element) "Movable")
    (`self.K2_SetActorLocation` _array_element (+ (`self.K2_GetActorLocation` _array_element) (`KismetMathLibrary.MakeVector` (`KismetMathLibrary.Lerp` (.x (`self.TranslationRandomizationMin`)) (.x (`self.TranslationRandomizationMax`)) (`KismetMathLibrary.RandomFloat`)) (`KismetMathLibrary.Lerp` (.y (`self.TranslationRandomizationMin`)) (.y (`self.TranslationRandomizationMax`)) (`KismetMathLibrary.RandomFloat`)) (`KismetMathLibrary.Lerp` (.z (`self.TranslationRandomizationMin`)) (.z (`self.TranslationRandomizationMax`)) (`KismetMathLibrary.RandomFloat`)))) false true)
    (`self.K2_SetActorRotation` _array_element (`KismetMathLibrary.ComposeRotators` (`self.K2_GetActorRotation` _array_element) (`KismetMathLibrary.MakeRotationFromAxes` (`KismetMathLibrary.VLerp` _x _x_2 (`KismetMathLibrary.RandomFloat`)) (`KismetMathLibrary.VLerp` _y _y_2 (`KismetMathLibrary.RandomFloat`)) (`KismetMathLibrary.VLerp` _z _z_2 (`KismetMathLibrary.RandomFloat`)))) false)
    (`self.SetActorScale3D` _array_element (* (`self.GetActorScale3D` _array_element) (`KismetMathLibrary.Lerp` (`self.ScaleRandomizationMin`) (`self.ScaleRandomizationMax`) (`KismetMathLibrary.RandomFloat`))))))

(fn `UserConstructionScript`)
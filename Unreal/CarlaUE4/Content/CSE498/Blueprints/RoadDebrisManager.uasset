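; Manager actor that scatters small and large debris over road meshes tagged with RoadTag, through functions with no callers in its own graphs.
; Small debris attaches a Niagara system to each tagged StaticMeshActor, clearing previous emitters first.
; Large debris fires randomized line traces within set bounds, spawning randomly yawed actors where they hit road.
; Both track spawns in arrays for removal, but large spawning does not clear earlier actors.
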(fn `ClearLargeDebris`
  (bind (_arrayindex _arrayelement) (`/Engine/EditorBlueprintResources/StandardMacros.ReverseForEachLoop` (`self.SpawnedLargeDebrisActors`))
    (:`LoopBody`
      (`self.K2_DestroyActor` _arrayelement))
    (:`Completed`
      (`KismetArrayLibrary.Array_Clear` (`self.SpawnedLargeDebrisActors`)))))

(fn `ClearSmallDebris`
  (bind (_arrayindex _arrayelement) (`/Engine/EditorBlueprintResources/StandardMacros.ReverseForEachLoop` (`self.SpawnedSmallDebrisEmitters`))
    (:`LoopBody`
      (`ActorComponent.K2_DestroyComponent` _arrayelement))
    (:`Completed`
      (`KismetArrayLibrary.Array_Clear` (`self.SpawnedSmallDebrisEmitters`)))))

(fn `SpawnLargeDebris`
  (locals (LineTraceObjectTypes :type "Array of EObjectTypeQuery Enum"))
  (bind (_x _y) (`KismetMathLibrary.BreakVector2D` (`self.LargeDebrisLineTraceMinXY`)))
  (bind (_x_2 _y_2) (`KismetMathLibrary.BreakVector2D` (`self.LargeDebrisLineTraceMaxXY`)))
  (bind (_x_3 _y_3) (`KismetMathLibrary.BreakVector2D` (`self.LargeDebrisLineTraceHeightRange`)))
  (bind _returnvalue (`KismetMathLibrary.RandomFloatInRange` _x _x_2))
  (bind _returnvalue_2 (`KismetMathLibrary.RandomFloatInRange` _y _y_2))
  (for _ (range (+ (`self.LargeDebrisSpawnAttempts`) 1))
    (bind (_outhit _returnvalue_3) (`KismetSystemLibrary.LineTraceSingleForObjects` (`KismetMathLibrary.MakeVector` _returnvalue _returnvalue_2 _x_3) (`KismetMathLibrary.MakeVector` _returnvalue _returnvalue_2 _y_3) (`local.LineTraceObjectTypes`)))
    (if _returnvalue_3
      (bind (_bblockinghit _binitialoverlap _time _distance _location _impactpoint _normal _impactnormal _physmat _hitactor) (`GameplayStatics.BreakHitResult` _outhit))
      (if (`KismetArrayLibrary.Array_Contains` (`Actor.Tags` _hitactor) (`self.RoadTag`))
        (bind _returnvalue_4 (`|SpawnActorFromClass` (`self.LargeDebrisSpawnedBlueprint`) (`KismetMathLibrary.MakeTransform` _location) "Undefined" "OverrideRootScale" null null))
        (`self.K2_AddActorLocalRotation` _returnvalue_4 (`KismetMathLibrary.MakeRotator` 0.0 0.0 (`KismetMathLibrary.RandomFloatInRange` 0.0 360.0)) false false)
        (`KismetArrayLibrary.Array_Add` (`self.SpawnedLargeDebrisActors`) _returnvalue_4))))
  (`KismetSystemLibrary.PrintString` "Spawned large debris:")
  (`KismetSystemLibrary.PrintString` (`KismetStringLibrary.Conv_IntToString` (`KismetArrayLibrary.Array_Length` (`self.SpawnedLargeDebrisActors`)))))

(fn `SpawnSmallDebris`
  (locals (CurrentRoad :type "StaticMeshActor Object Reference"))
  (`self.ClearSmallDebris`)
  (bind _outactors (`GameplayStatics.GetAllActorsOfClassWithTag` "/Script/Engine.StaticMeshActor" (`self.RoadTag`)))
  (for _array_element _outactors
    (bind _returnvalue (`NiagaraFunctionLibrary.SpawnSystemAttached` "/Game/CSE498/Blueprints/SmallRoadDebris.SmallRoadDebris" (`StaticMeshActor.StaticMeshComponent` _array_element) "None" (0.0 0.0 0.0) (struct) "KeepRelativeOffset"))
    (`KismetArrayLibrary.Array_Add` (`self.SpawnedSmallDebrisEmitters`) _returnvalue)))

(fn `UserConstructionScript`)
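; BuildingParameterizer varies static mesh props in a Carla scene (buildings, hydrants, light boxes, street lights, trees) by scale, location, rotation and mesh.
; BeginPlay caches original transforms and meshes and maps categories to content folders.
; Set or randomize functions reset to those originals, then edit actors matched by name substring or ActorToMove tag, drawing random meshes from the Asset Registry.
; Weighted scale randomization and SaveGame persistence of offsets are included.
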(event `self.ReceiveBeginPlay`
  (bind _categorymap (`self.CategoryMap`))
  (bind _outactors (`GameplayStatics.GetAllActorsOfClass` "/Script/Engine.StaticMeshActor"))
  (for _array_element _outactors
    (if (not (`KismetMathLibrary.ClassIsChildOf` (`GameplayStatics.GetObjectClass` _array_element) "/Script/Engine.Light"))
      (`KismetArrayLibrary.Array_Add` (`self.OriginalMeshScale`) (`self.GetActorScale3D` _array_element))
      (`KismetArrayLibrary.Array_Add` (`self.OriginalMeshRotation`) (`self.K2_GetActorRotation` _array_element))
      (`KismetArrayLibrary.Array_Add` (`self.OriginalMeshLocation`) (`self.K2_GetActorLocation` _array_element))
      (`KismetArrayLibrary.Array_Add` (`self.OriginalMeshes`) (`StaticMeshComponent.StaticMesh` (`self.GetComponentByClass` _array_element "/Script/Engine.StaticMeshComponent")))
      (bind _returnvalue (`KismetSystemLibrary.GetObjectName` _array_element))
      (if (and (`KismetStringLibrary.Contains` _returnvalue "FireHydrant") (not (`BlueprintMapLibrary.Map_Contains` _categorymap "FireHydrant")))
        (`BlueprintMapLibrary.Map_Add` _categorymap "FireHydrant" "/Game/Carla/Static/Static")
        (elif (and (`KismetStringLibrary.Contains` _returnvalue "LightBox") (not (`BlueprintMapLibrary.Map_Contains` _categorymap "LightBox")))
          (`BlueprintMapLibrary.Map_Add` _categorymap "LightBox" "/Game/Carla/Static/Static")
          (elif (and (`KismetStringLibrary.Contains` _returnvalue "StreetLight") (not (`BlueprintMapLibrary.Map_Contains` _categorymap "StreetLight")))
            (`BlueprintMapLibrary.Map_Add` _categorymap "StreetLight" "/Game/Carla/Static/StreetLight")
            (elif (and (`KismetStringLibrary.Contains` _returnvalue "TreeSpawn") (not (`BlueprintMapLibrary.Map_Contains` _categorymap "TreeSpawn")))
              (`BlueprintMapLibrary.Map_Add` _categorymap "TreeSpawn" "/Game/Carla/Static/Vegetation/Trees")
              (elif (and (not (`BlueprintMapLibrary.Map_Contains` _categorymap "Building")) (`self.ActorHasTag` _array_element "ActorToMove"))
                (`BlueprintMapLibrary.Map_Add` _categorymap "Building" "/Game/Carla/Static/Building")))))))))

(fn `AssetMeshChanger`
  (`self.ResetMesh`)
  (bind _outactors (`GameplayStatics.GetAllActorsOfClass` "/Script/Engine.StaticMeshActor"))
  (for _array_element _outactors
    (bind _returnvalue (`KismetSystemLibrary.GetObjectName` _array_element))
    (if (and (not (`KismetStringLibrary.Contains` _returnvalue "Light")) (>= (`KismetStringLibrary.FindSubstring` _returnvalue (`self.Asset Category`)) 0))
      (`StaticMeshComponent.SetStaticMesh` (`StaticMeshActor.StaticMeshComponent` _array_element) (`self.CurrentMesh`)))))

(fn `AssetRotator`
  (`self.Reset Rotation`)
  (bind _outactors (`GameplayStatics.GetAllActorsOfClass` "/Script/Engine.StaticMeshActor"))
  (for _array_element _outactors
    (bind _returnvalue (`KismetSystemLibrary.GetObjectName` _array_element))
    (if (and (>= (`KismetStringLibrary.FindSubstring` _returnvalue (`self.Asset Category`)) 0) (not (`KismetStringLibrary.Contains` _returnvalue "Light")))
      (`SceneComponent.SetMobility` (`Actor.RootComponent` _array_element) "Movable")
      (`self.K2_SetActorRotation` _array_element (`KismetMathLibrary.ComposeRotators` (`self.K2_GetActorRotation` _array_element) (`self.RotateBy`)) false))))

(fn `AssetScaler`
  (`self.ResetScale`)
  (bind _outactors (`GameplayStatics.GetAllActorsOfClass` "/Script/Engine.StaticMeshActor"))
  (for _array_element _outactors
    (if (>= (`KismetStringLibrary.FindSubstring` (`KismetSystemLibrary.GetObjectName` _array_element) (`self.Asset Category`)) 0)
      (bind _returnvalue (`KismetMathLibrary.MakeVector` (* (.x (`self.GetActorScale3D` _array_element)) (.x (`self.ScaleBy`))) (* (.y (`self.GetActorScale3D` _array_element)) (.y (`self.ScaleBy`))) (* (.z (`self.GetActorScale3D` _array_element)) (.z (`self.ScaleBy`)))))
      (`SceneComponent.SetWorldScale3D` (`Actor.RootComponent` _array_element) _returnvalue)
      (set `self.CurrentScales` (`|MakeArray` _returnvalue)))))

(fn `AssetTranslate`
  (`self.ResetLocation`)
  (bind _outactors (`GameplayStatics.GetAllActorsOfClass` "/Script/Engine.StaticMeshActor"))
  (for _array_element _outactors
    (bind _returnvalue (`KismetSystemLibrary.GetObjectName` _array_element))
    (if (and (not (`KismetStringLibrary.Contains` _returnvalue "Light")) (>= (`KismetStringLibrary.FindSubstring` _returnvalue (`self.Asset Category`)) 0))
      (bind _returnvalue_2 (`KismetMathLibrary.MakeVector` (+ (.x (`self.K2_GetActorLocation` _array_element)) (.x (`self.MoveTo`))) (+ (.y (`self.K2_GetActorLocation` _array_element)) (.y (`self.MoveTo`))) (+ (.z (`self.K2_GetActorLocation` _array_element)) (.z (`self.MoveTo`)))))
      (`SceneComponent.K2_SetWorldLocation` (`Actor.RootComponent` _array_element) _returnvalue_2 false true)
      (set `self.CurrentLocations` (`|MakeArray` _returnvalue_2)))))

(fn `BuildingScaler`
  (`self.ResetScale`)
  (bind _outactors (`GameplayStatics.GetAllActorsWithTag` "ActorToMove"))
  (for _array_element _outactors
    (`SceneComponent.SetWorldScale3D` (`Actor.RootComponent` _array_element) (`KismetMathLibrary.MakeVector` (* (.x (`self.GetActorScale3D` _array_element)) (.x (`self.ScaleBy`))) (* (.y (`self.GetActorScale3D` _array_element)) (.y (`self.ScaleBy`))) (* (.z (`self.GetActorScale3D` _array_element)) (.z (`self.ScaleBy`)))))))

(fn `DetermineIndex`
  (params (RandomValue :type "Float (double-precision)"))
  (returns (IndexThatWon :type Integer))
  (locals (LocalSum :type "Float (double-precision)"))
  (for (_array_element _array_index) (`self.WeightValues`)
    (bind _output_get (set `local.LocalSum` (+ (`local.LocalSum`) _array_element)))
    (if (>= _output_get RandomValue)
      (break)))
  (return _array_index))

(fn `LoadState`
  (bind _slot_save_name (`self.Slot Save Name`))
  (bind _returnvalue (`GameplayStatics.DoesSaveGameExist` _slot_save_name))
  (if _returnvalue
    (bind _returnvalue_2 (`GameplayStatics.LoadGameFromSlot` _slot_save_name))
    (bind _asbp_save (cast `/Game/CSE498/Blueprints/BP_Save` _returnvalue_2))
    (`self.ResetLocation`)
    (`self.Reset Rotation`)
    (`self.ResetScale`)
    (bind _output_get (set `self.MoveTo` (`/Game/CSE498/Blueprints/BP_Save.Location` _asbp_save)))
    (bind _output_get_2 (set `self.RotateBy` (`/Game/CSE498/Blueprints/BP_Save.Rotation` _asbp_save)))
    (bind _output_get_3 (set `self.ScaleBy` (`/Game/CSE498/Blueprints/BP_Save.Scale` _asbp_save)))
    (bind _output_get_4 (set `self.Asset Category` (`/Game/CSE498/Blueprints/BP_Save.AssetCategory` _asbp_save)))
    (bind _outactors (`GameplayStatics.GetAllActorsOfClass` "/Script/Engine.StaticMeshActor"))
    (for _array_element _outactors
      (bind _returnvalue_3 (`KismetSystemLibrary.GetObjectName` _array_element))
      (if (and (not (`KismetStringLibrary.Contains` _returnvalue_3 "Light")) (>= (`KismetStringLibrary.FindSubstring` _returnvalue_3 _output_get_4) 0))
        (`self.K2_SetActorLocation` _array_element (`KismetMathLibrary.MakeVector` (+ (.x (`self.K2_GetActorLocation` _array_element)) (.x _output_get)) (+ (.y (`self.K2_GetActorLocation` _array_element)) (.y _output_get)) (+ (.z (`self.K2_GetActorLocation` _array_element)) (.z _output_get))) false false)
        (`self.K2_SetActorRotation` _array_element (`KismetMathLibrary.ComposeRotators` (`self.K2_GetActorRotation` _array_element) _output_get_2) false)
        (`SceneComponent.SetWorldScale3D` (`Actor.RootComponent` _array_element) (`KismetMathLibrary.MakeVector` (* (.x (`self.GetActorScale3D` _array_element)) (.x _output_get_3)) (* (.y (`self.GetActorScale3D` _array_element)) (.y _output_get_3)) (* (.z (`self.GetActorScale3D` _array_element)) (.z _output_get_3))))))))

(fn `RandomizeBuildingScale`
  (params (scale_max :type "Float (double-precision)"))
  (`self.ResetScale`)
  (bind _outactors (`GameplayStatics.GetAllActorsWithTag` "ActorToMove"))
  (for _array_element _outactors
    (bind _returnvalue (`KismetMathLibrary.MakeVector` (* (.x (`self.GetActorScale3D` _array_element)) (`KismetMathLibrary.Lerp` (.x (`self.MinScaleBy`)) scale_max (`KismetMathLibrary.RandomFloat`))) (* (.y (`self.GetActorScale3D` _array_element)) (`KismetMathLibrary.Lerp` (.y (`self.MinScaleBy`)) scale_max (`KismetMathLibrary.RandomFloat`))) (* (.z (`self.GetActorScale3D` _array_element)) (`KismetMathLibrary.Lerp` (.z (`self.MinScaleBy`)) scale_max (`KismetMathLibrary.RandomFloat`)))))
    (`SceneComponent.SetWorldScale3D` (`Actor.RootComponent` _array_element) _returnvalue)
    (set `self.ScaleBy` _returnvalue)))

(fn `RandomizeLocation`
  (params (AssetCat :type String))
  (bind _output_get (set `self.Asset Category` AssetCat))
  (`self.ResetLocation`)
  (bind _outactors (`GameplayStatics.GetAllActorsOfClass` "/Script/Engine.StaticMeshActor"))
  (for _array_element _outactors
    (bind _returnvalue (`KismetSystemLibrary.GetObjectName` _array_element))
    (if (and (not (`KismetStringLibrary.Contains` _returnvalue "Light")) (>= (`KismetStringLibrary.FindSubstring` _returnvalue _output_get) 0))
      (bind _returnvalue_2 (+ (`self.K2_GetActorLocation` _array_element) (`KismetMathLibrary.MakeVector` (`KismetMathLibrary.Lerp` (.x (`self.MinMove`)) (.x (`self.MaxMove`)) (`KismetMathLibrary.RandomFloat`)) (`KismetMathLibrary.Lerp` (.y (`self.MinMove`)) (.y (`self.MaxMove`)) (`KismetMathLibrary.RandomFloat`)) (`KismetMathLibrary.Lerp` (.z (`self.MinMove`)) (.z (`self.MaxMove`)) (`KismetMathLibrary.RandomFloat`)))))
      (`SceneComponent.K2_SetWorldLocation` (`Actor.RootComponent` _array_element) _returnvalue_2 false true)
      (set `self.CurrentLocations` (`|MakeArray` _returnvalue_2)))))

(fn `RandomizeMesh`
  (params (AssetCat :type String))
  (locals (`Package Path` :type Name))
  (bind _output_get (set `self.Asset Category` AssetCat))
  (`self.ResetMesh`)
  (bind _outactors (`GameplayStatics.GetAllActorsOfClass` "/Script/Engine.StaticMeshActor"))
  (for _array_element _outactors
    (bind _asstatic_mesh_actor (cast `StaticMeshActor` _array_element))
    (bind _returnvalue (`KismetSystemLibrary.GetObjectName` _array_element))
    (if (and (not (`KismetStringLibrary.Contains` _returnvalue "Light")) (>= (`KismetStringLibrary.FindSubstring` _returnvalue _output_get) 0))
      (if (and (`self.ActorHasTag` _asstatic_mesh_actor "ActorToMove") (`KismetStringLibrary.Contains` _output_get "Building"))
        (break)
        (else
          (bind _outassetdata (message `AssetRegistry.GetAssetsByPath` (`KismetSystemLibrary.Conv_InterfaceToObject` (`AssetRegistryHelpers.GetAssetRegistry`)) (`BlueprintMapLibrary.Map_Find` (`self.CategoryMap`) _output_get) false false))
          (bind _asstatic_mesh (cast `StaticMesh` (`AssetRegistryHelpers.GetAsset` (`KismetArrayLibrary.Array_Random` _outassetdata))))
          (`StaticMeshComponent.SetStaticMesh` (`StaticMeshActor.StaticMeshComponent` _asstatic_mesh_actor) _asstatic_mesh)))))
  (bind _outactors_2 (`GameplayStatics.GetAllActorsWithTag` "ActorToMove"))
  (for _array_element_2 _outactors_2
    (bind _asstatic_mesh_actor_2 (cast `StaticMeshActor` _array_element_2))
    (bind _returnvalue_2 (`KismetSystemLibrary.GetObjectName` _array_element_2))
    (if (not (or (`KismetStringLibrary.Contains` _returnvalue_2 "Light") (`KismetStringLibrary.Contains` _returnvalue_2 "TreeSpawn") (`KismetStringLibrary.Contains` _returnvalue_2 "FireHydrant") (`KismetStringLibrary.Contains` _returnvalue_2 "LightBox") (`KismetStringLibrary.Contains` _returnvalue_2 "StreetLight")))
      (bind _outassetdata_2 (message `AssetRegistry.GetAssetsByPath` (`KismetSystemLibrary.Conv_InterfaceToObject` (`AssetRegistryHelpers.GetAssetRegistry`)) (`BlueprintMapLibrary.Map_Find` (`self.CategoryMap`) "Building") false false))
      (bind _asstatic_mesh_2 (cast `StaticMesh` (`AssetRegistryHelpers.GetAsset` (`KismetArrayLibrary.Array_Random` _outassetdata_2))))
      (`StaticMeshComponent.SetStaticMesh` (`StaticMeshActor.StaticMeshComponent` _asstatic_mesh_actor_2) _asstatic_mesh_2))))

(fn `RandomizeRotate`
  (params (AssetCat :type String))
  (bind (_x _y _z) (`KismetMathLibrary.BreakRotIntoAxes` (`self.MinRotateBy`)))
  (bind (_x_2 _y_2 _z_2) (`KismetMathLibrary.BreakRotIntoAxes` (`self.MaxRotateBy`)))
  (bind _returnvalue (`KismetMathLibrary.MakeRotationFromAxes` (`KismetMathLibrary.VLerp` _x _x_2 (`KismetMathLibrary.RandomFloat`)) (`KismetMathLibrary.VLerp` _y _y_2 (`KismetMathLibrary.RandomFloat`)) (`KismetMathLibrary.VLerp` _z _z_2 (`KismetMathLibrary.RandomFloat`))))
  (bind _output_get (set `self.Asset Category` AssetCat))
  (`self.Reset Rotation`)
  (bind _outactors (`GameplayStatics.GetAllActorsOfClass` "/Script/Engine.StaticMeshActor"))
  (for _array_element _outactors
    (bind _returnvalue_2 (`KismetSystemLibrary.GetObjectName` _array_element))
    (if (and (>= (`KismetStringLibrary.FindSubstring` _returnvalue_2 _output_get) 0) (not (`KismetStringLibrary.Contains` _returnvalue_2 "Light")))
      (`SceneComponent.SetMobility` (`Actor.RootComponent` _array_element) "Movable")
      (`self.K2_SetActorRotation` _array_element (`KismetMathLibrary.ComposeRotators` (`self.K2_GetActorRotation` _array_element) _returnvalue) false)
      (set `self.RotateBy` _returnvalue))))

(fn `RandomizeScale`
  (params (AssetCat :type String))
  (bind _output_get (set `self.Asset Category` AssetCat))
  (`self.ResetScale`)
  (bind _outactors (`GameplayStatics.GetAllActorsOfClass` "/Script/Engine.StaticMeshActor"))
  (for _array_element _outactors
    (if (>= (`KismetStringLibrary.FindSubstring` (`KismetSystemLibrary.GetObjectName` _array_element) _output_get) 0)
      (bind _returnvalue (* (`self.GetActorScale3D` _array_element) (`KismetMathLibrary.MakeVector` (`KismetMathLibrary.Lerp` (.x (`self.MinScaleBy`)) (.x (`self.MaxScaleBy`)) (`KismetMathLibrary.RandomFloat`)) (`KismetMathLibrary.Lerp` (.y (`self.MinScaleBy`)) (.y (`self.MaxScaleBy`)) (`KismetMathLibrary.RandomFloat`)) (`KismetMathLibrary.Lerp` (.z (`self.MinScaleBy`)) (.z (`self.MaxScaleBy`)) (`KismetMathLibrary.RandomFloat`)))))
      (`SceneComponent.SetWorldScale3D` (`Actor.RootComponent` _array_element) _returnvalue)
      (set `self.ScaleBy` _returnvalue))))

(fn `Reset Rotation`
  (bind _outactors (`GameplayStatics.GetAllActorsOfClass` "/Script/Engine.StaticMeshActor"))
  (for (_array_element _array_index) _outactors
    (if (not (`KismetMathLibrary.ClassIsChildOf` (`GameplayStatics.GetObjectClass` _array_element) "/Script/Engine.Light"))
      (`SceneComponent.SetMobility` (`Actor.RootComponent` _array_element) "Movable")
      (`self.K2_SetActorRotation` _array_element (`|GetArrayItem` (`self.OriginalMeshRotation`) _array_index) false))))

(fn `ResetLocation`
  (bind _outactors (`GameplayStatics.GetAllActorsOfClass` "/Script/Engine.StaticMeshActor"))
  (for (_array_element _array_index) _outactors
    (if (not (`KismetMathLibrary.ClassIsChildOf` (`GameplayStatics.GetObjectClass` _array_element) "/Script/Engine.Light"))
      (bind _rootcomponent (`Actor.RootComponent` _array_element))
      (`SceneComponent.SetMobility` _rootcomponent "Movable")
      (`SceneComponent.K2_SetWorldLocation` _rootcomponent (`|GetArrayItem` (`self.OriginalMeshLocation`) _array_index) false true))))

(fn `ResetMesh`
  (bind _outactors (`GameplayStatics.GetAllActorsOfClass` "/Script/Engine.StaticMeshActor"))
  (for (_array_element _array_index) _outactors
    (bind _staticmeshcomponent (`StaticMeshActor.StaticMeshComponent` _array_element))
    (`SceneComponent.SetMobility` _staticmeshcomponent "Movable")
    (`StaticMeshComponent.SetStaticMesh` _staticmeshcomponent (`|GetArrayItem` (`self.OriginalMeshes`) _array_index))))

(fn `ResetScale`
  (bind _outactors (`GameplayStatics.GetAllActorsOfClass` "/Script/Engine.StaticMeshActor"))
  (for (_array_element _array_index) _outactors
    (`SceneComponent.SetWorldScale3D` (`Actor.RootComponent` _array_element) (`|GetArrayItem` (`self.OriginalMeshScale`) _array_index))))

(fn `SaveState`
  (bind _returnvalue (`GameplayStatics.DoesSaveGameExist` (`self.Slot Save Name`)))
  (if _returnvalue
    (`GameplayStatics.LoadGameFromSlot` (`self.Slot Save Name`))
    (else
      (bind _returnvalue_2 (`GameplayStatics.CreateSaveGameObject` "/Game/CSE498/Blueprints/BP_Save.BP_Save_C"))))
  (bind _output_get (set `self.Save_REF` _returnvalue_2))
  (bind _asbp_save (cast `/Game/CSE498/Blueprints/BP_Save` _output_get))
  (set `/Game/CSE498/Blueprints/BP_Save.CurrentScales` (`self.CurrentScales`) _asbp_save)
  (set `/Game/CSE498/Blueprints/BP_Save.Scale` (`self.ScaleBy`) _asbp_save)
  (set `/Game/CSE498/Blueprints/BP_Save.Location` (`self.MoveTo`) _asbp_save)
  (set `/Game/CSE498/Blueprints/BP_Save.Rotation` (`self.RotateBy`) _asbp_save)
  (set `/Game/CSE498/Blueprints/BP_Save.AssetCategory` (`self.Asset Category`) _asbp_save)
  (`GameplayStatics.SaveGameToSlot` (`self.Save_REF`) (`self.Slot Save Name`)))

(fn `SumValues`
  (returns (SumOfValues :type "Float (double-precision)"))
  (locals (LocalSum :type "Float (double-precision)"))
  (for _array_element (`self.WeightValues`)
    (set `local.LocalSum` (+ (`local.LocalSum`) _array_element)))
  (return (`local.LocalSum`)))

(fn `UserConstructionScript`)

(fn `WeightedRandomizeBuildingScale`
  (bind _sumofvalues (`self.SumValues`))
  (bind _indexthatwon (`self.DetermineIndex` (`KismetMathLibrary.RandomFloatInRange` 0.0 _sumofvalues)))
  (`self.RandomizeBuildingScale` (`|GetArrayItem` (`self.WeightAbilities`) _indexthatwon)))